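; BP_SpawnRoad is a moving road actor that also holds logic for spawning straight road pieces.
; On Tick, once BP_GameModeBase reports IsStart, it moves along its forward vector by SpawnRoadSpeed scaled by delta time.
; SpawnRoadGo accumulates time and spawns BP_Spawn_StraightGo_Road at StartRoadArrow whenever DelayTime is reached, though no graph in this Blueprint calls it.
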(event `self.ReceiveTick`
  (params (DeltaSeconds :type "Float (single-precision)"))
  ;[1 1 1] (길)액터가 (-x축)으로 초당 (-200)이동하게
  (bind _asbp_game_mode_base (cast `/Game/Blueprints/GameMode/BP_GameModeBase` (`GameplayStatics.GetGameMode`)))
  (if (`/Game/Blueprints/GameMode/BP_GameModeBase.IsStart` _asbp_game_mode_base)
    (`self.K2_SetActorLocation` (+ (`self.K2_GetActorLocation`) (* (* (`self.GetActorForwardVector`) (`self.SpawnRoadSpeed`)) DeltaSeconds)))))

(event `self.ReceiveActorBeginOverlap`
  (params (OtherActor :type "Actor Object Reference")))

(fn `SpawnRoad_go`
  (params (A :type "Float (double-precision)"))
  (bind _output_get (set `self.CurrentTime` (+ A (`self.CurrentTime`))))
  (if (>= _output_get (`self.DelayTime`))
    (`|SpawnActorFromClass` "/Game/Blueprints/BP_Spawn_StraightGo_Road.BP_Spawn_StraightGo_Road_C" (`SceneComponent.K2_GetComponentToWorld` (`self.StartRoadArrow`)) "Undefined" "MultiplyWithRoot" null null)
    (set `self.CurrentTime` 0.0)))

(fn `UserConstructionScript`)