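; Player character Blueprint that shows the in-game UMG widget on BeginPlay and steps sideways along Y by MoveRange on A/D, with Space to jump.
; While the game mode's IsStart is set, Tick plays a smooth-start timeline that accumulates Speed and adds downward movement input.
; Speed is not applied to movement here.
; Older Speed-ramp and X-axis step logic remains disconnected.
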(event `self.ReceiveTick`
  (params (DeltaSeconds :type "Float (single-precision)"))
  (bind _asbp_game_mode_base (cast `/Game/Blueprints/BP_GameModeBase` (`GameplayStatics.GetGameMode`)))
  (if (`/Game/Blueprints/BP_GameModeBase.IsStart` _asbp_game_mode_base)
    (bind (_direction `_부드러운_시작모션`) (`Timeline|타임라인` :`NewTime` DeltaSeconds :!label _label)
      (:`Update`
        (set `self.Speed` (+ `_부드러운_시작모션` (`self.Speed`)))
        (`self.AddMovementInput` (0.0 0.0 -1.0))))
    (else
      (goto _label :!via `Stop`))))

(event `Key|A`
  (params (Key :type "Key Structure"))
  (:`Pressed`
    (`self.K2_SetActorLocation` (+ (`self.K2_GetActorLocation`) (* (`KismetMathLibrary.MakeVector` 0.0 (`self.MoveRange`)) (0.0 -1.0 0.0))))))

(event `Key|D`
  (params (Key :type "Key Structure"))
  (:`Pressed`
    (`self.K2_SetActorLocation` (+ (`self.K2_GetActorLocation`) (* (`KismetMathLibrary.MakeVector` 0.0 (`self.MoveRange`)) (0.0 1.0 0.0))))))

(event `self.ReceiveBeginPlay`
  (`|ExecutionSequence`
    (:`then_0`
      (bind _returnvalue (`|CreateWidget` "/Game/UMG/UMG_InGameing_Widget.UMG_InGameing_Widget_C"))
      (`UserWidget.AddToViewport` _returnvalue 0))))

(event `Key|SpaceBar`
  (params (Key :type "Key Structure"))
  (:`Pressed`
    (`self.Jump`)))

(fn `UserConstructionScript`)