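; Game mode that tracks a score built from survival time and collected coins, and keeps the best result.
; After a short start delay, it sets IsStart and opens a gate that lets Tick accumulate time and recompute the score with a coin bonus.
; AddCoin raises the coin count.
; BestTime, despite its name, holds the high score, loaded at BeginPlay and saved through BP_SaveScore whenever beaten during Tick.
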(event `self.ReceiveBeginPlay`
  (bind _bestscore (`self.LoadScoreData`))
  (set `self.BestTime` _bestscore)
  (`KismetSystemLibrary.Delay` 3.0)
  (set `self.IsStart` true)
  (goto _label :!via `Open`))

(event `self.ReceiveTick`
  (params (DeltaSeconds :type "Float (single-precision)"))
  (`/Engine/EditorBlueprintResources/StandardMacros.Gate` true :!label _label
    (:`Exit`
      (bind _output_get (set `self.CurrentTime` (+ DeltaSeconds (`self.CurrentTime`))))
      (bind _returnvalue (+ _output_get (* (`self.CoinNum`) 100)))
      (set `self.NowScore` (`KismetMathLibrary.FTrunc` _returnvalue))
      (if (> _returnvalue (`self.BestTime`))
        (bind _output_get_2 (set `self.BestTime` (`KismetMathLibrary.FTrunc` _returnvalue)))
        (`self.SaveScoreData` _output_get_2)))))

(fn `AddCoin`
  (params (GetCoin :type Integer))
  (set `self.CoinNum` (+ GetCoin (`self.CoinNum`))))

(fn `LoadScoreData`
  (returns (BestScore :type Integer))
  (bind _returnvalue (`GameplayStatics.DoesSaveGameExist` (`self.Slot Name`)))
  (if _returnvalue
    (bind _returnvalue_2 (`GameplayStatics.LoadGameFromSlot` (`self.Slot Name`)))
    (bind _asbp_save_score (cast `/Game/Blueprints/GameSaves/BP_SaveScore` _returnvalue_2))
    (return (`/Game/Blueprints/GameSaves/BP_SaveScore.ScoreData` _asbp_save_score))))

(fn `SaveScoreData`
  (params (SaveValue :type Integer))
  (bind _returnvalue (`GameplayStatics.CreateSaveGameObject` "/Game/Blueprints/GameSaves/BP_SaveScore.BP_SaveScore_C"))
  (bind _output_get (set `self.SaveInstance` _returnvalue))
  (set `/Game/Blueprints/GameSaves/BP_SaveScore.ScoreData` SaveValue _output_get)
  (`GameplayStatics.SaveGameToSlot` _output_get (`self.Slot Name`)))

(fn `UserConstructionScript`)