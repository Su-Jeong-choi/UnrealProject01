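; BP_SpawnRoad_StraightGo is a straight road segment that moves itself and spawns its own successor, forming a chain of road pieces.
; Tick moves the actor along its forward vector at SpawnRoadSpeed while accumulating CurrentTime.
; Once DelayTime elapses, a DoOnce spawns another instance at RunDirArrow's transform, so each segment spawns only one.
; SpawnRoadGo repeats the timed spawn logic without the DoOnce, but Tick does not call it.
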(event `self.ReceiveTick`
  (params (DeltaSeconds :type "Float (single-precision)"))
  (`|ExecutionSequence`
    (:`then_0`
      (`self.K2_SetActorLocation` (+ (`self.K2_GetActorLocation`) (* (* (`self.GetActorForwardVector`) (`self.SpawnRoadSpeed`)) DeltaSeconds))))
    (:`then_1`
      (bind _output_get (set `self.CurrentTime` (+ DeltaSeconds (`self.CurrentTime`))))
      (if (>= _output_get (`self.DelayTime`))
        (`/Engine/EditorBlueprintResources/StandardMacros.DoOnce` false
          (:`Completed`
            (`|SpawnActorFromClass` "BP_SpawnRoad_StraightGo_C" (`SceneComponent.K2_GetComponentToWorld` (`self.RunDirArrow`)) "Undefined" "MultiplyWithRoot" null null)
            (set `self.CurrentTime` 0.0)))))))

(fn `SpawnRoad_go`
  (params (A :type "Float (double-precision)"))
  (bind _output_get (set `self.CurrentTime` (+ A (`self.CurrentTime`))))
  (if (>= _output_get (`self.DelayTime`))
    (`|SpawnActorFromClass` "BP_SpawnRoad_StraightGo_C" (`SceneComponent.K2_GetComponentToWorld` (`self.RunDirArrow`)) "Undefined" "MultiplyWithRoot" null null)
    (set `self.CurrentTime` 0.0)))

(fn `UserConstructionScript`)