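; Coin pickup that spins, moves with the scrolling road and adds to the player's coin count.
; Tick rotates the Scene component by a fixed per-frame yaw and, while BP_GameModeBase's IsStart is set, moves the actor along its forward vector at SpawnRoadSpeed, scaled by delta time.
; Any sphere overlap destroys the coin, but only a BP_CharPlayer overlap calls AddCoin on the game mode and prints a debug message.
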(event `self.ReceiveBeginPlay`)

(event `self.ReceiveActorBeginOverlap`
  (params (OtherActor :type "Actor Object Reference")))

(event `self.ReceiveTick`
  (params (DeltaSeconds :type "Float (single-precision)"))
  (`|ExecutionSequence`
    (:`then_0`
      (`SceneComponent.K2_AddRelativeRotation` (`self.Scene`) (`KismetMathLibrary.MakeRotator` 0.0 0.0 1.0) false false))
    (:`then_1`
      ;[1 1 1] (길)액터가 (-x축)으로 초당 (-200)이동하게
      (bind _asbp_game_mode_base (cast `/Game/Blueprints/BP_GameModeBase` (`GameplayStatics.GetGameMode`)))
      (if (`/Game/Blueprints/BP_GameModeBase.IsStart` _asbp_game_mode_base)
        (`self.K2_SetActorLocation` (+ (`self.K2_GetActorLocation`) (* (* (`self.GetActorForwardVector`) (`self.SpawnRoadSpeed`)) DeltaSeconds)))))))

(event `self.SphereCollision.OnComponentBeginOverlap`
  (params (OverlappedComponent :type "PrimitiveComponent Object Reference") (OtherActor :type "Actor Object Reference") (OtherComp :type "PrimitiveComponent Object Reference") (OtherBodyIndex :type Integer) (bFromSweep :type Boolean) (SweepResult :type "HitResult Structure (by ref)"))
  (`self.K2_DestroyActor`)
  (cast `/Game/Blueprints/BP_CharPlayer` OtherActor)
  (`/Game/Blueprints/BP_GameModeBase.AddCoin` (cast `/Game/Blueprints/BP_GameModeBase` (`GameplayStatics.GetGameMode`) :!pure true) 1)
  (`KismetSystemLibrary.PrintString` "코인 먹음"))

(fn `StartRotation`
  (params (DeltaSecond :type "Float (double-precision)")))

(fn `UserConstructionScript`)